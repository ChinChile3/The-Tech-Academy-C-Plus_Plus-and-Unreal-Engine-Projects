(event Custom|UpdatePoints
  ;[1 1 1] Increment Point UI by 1
  (bind _output_get (Variables|Default|SetCurrentPoints (+ 1 (Variables|Default|GetCurrentPoints))))
  (Variables|/Game/Blueprints/BP_UserInterface.BP_UserInterface_C|SetPoint (Variables|Default|GetCurrentUI) _output_get)
  (CallFunction|EndGame))

(event Custom|EndGame
  ;[1 1 1] Checks PickUps Collected
  (if (>= (Variables|Default|GetCurrentPoints) 8)
    (Variables|/Game/Blueprints/BP_UserInterface.BP_UserInterface_C|SetYouWinOpacity (Variables|Default|GetCurrentUI) 1.0)))

(event EventBeginPlay
  ;[1 1 1] Adds UI to Screen
  (bind _returnvalue (UserInterface|CreateWidget "/Game/Blueprints/BP_UserInterface.BP_UserInterface_C"))
  (bind _output_get (Variables|Default|SetCurrentUI _returnvalue))
  (UserInterface|Viewport|AddtoViewport _output_get 0))

(fn ConstructionScript)