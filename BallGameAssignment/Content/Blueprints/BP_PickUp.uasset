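; BP_PickUp is a rotating collectible in a ball game that awards points when the ball touches it.
; On Tick it applies a local rotation from roll, pitch and yaw speed variables scaled by delta time.
; When a BP_Ball overlaps it, it destroys itself and then calls UpdatePoints on BP_BallGameMode.
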(event EventTick
  (params (DeltaSeconds :type Float%20%28single-precision%29))
  ;[1 1 1] Cube Rotation
  (Transformation|AddActorLocalRotation (* (Math|Rotator|MakeRotator (Variables|Default|GetRollSpeed) (Variables|Default|GetPitchSpeed) (Variables|Default|GetYawSpeed)) DeltaSeconds) false false))

(event Collision|EventActorBeginOverlap
  (params (OtherActor :type Actor%20Object%20Reference))
  ;[1 1 1] Destroyed upon contact
  (Utilities|Casting|CastToBP_Ball OtherActor)
  (Actor|DestroyActor)
  (bind _asbp_ball_game_mode (Utilities|Casting|CastToBP_BallGameMode (Game|GetGameMode)))
  (Default|UpdatePoints _asbp_ball_game_mode))

(fn ConstructionScript)